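; GM_Game is a game mode that spawns and possesses a BP_Player for each player as they log in.
; The first player spawns at the first PlayerStart found with PlayerID 1.
; Any later login spawns at the second PlayerStart with PlayerID 2, then starts the match timer on GS_MatchState, suggesting a two-player match.
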(event `self.K2_PostLogin`
  (params (NewPlayer :type "PlayerController Object Reference"))
  (bind _returnvalue (`self.GetNumPlayers`))
  (if (== _returnvalue 1)
    (bind _outactors (`GameplayStatics.GetAllActorsOfClass` "/Script/Engine.PlayerStart"))
    (bind _returnvalue_2 (`|SpawnActorFromClass` "/Game/HolySheep/Characters/Player/BP_Player.BP_Player_C" (`self.GetTransform` (`|GetArrayItem` _outactors)) "Undefined" "MultiplyWithRoot" NewPlayer null))
    (`Controller.Possess` NewPlayer _returnvalue_2)
    (set `/Game/HolySheep/Characters/Player/BP_Player.PlayerID` 1 _returnvalue_2)
    (else
      (bind _outactors_2 (`GameplayStatics.GetAllActorsOfClass` "/Script/Engine.PlayerStart"))
      (bind _returnvalue_3 (`|SpawnActorFromClass` "/Game/HolySheep/Characters/Player/BP_Player.BP_Player_C" (`self.GetTransform` (`|GetArrayItem` _outactors_2 1)) "Undefined" "MultiplyWithRoot" NewPlayer null))
      (`Controller.Possess` NewPlayer _returnvalue_3)
      (set `/Game/HolySheep/Characters/Player/BP_Player.PlayerID` 2 _returnvalue_3)
      (bind _asgs_match_state (cast `/Game/HolySheep/GameMode/GS_MatchState` (`GameplayStatics.GetGameState`)))
      (`/Game/HolySheep/GameMode/GS_MatchState.Start Timer` _asgs_match_state))))

(fn `UserConstructionScript`)